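; Door controller actor that swings a tagged door open or closed when the first-person player interacts.
; On BeginPlay it binds DoorStatus to the character's Interact event, which toggles IsOpen for the actor in the player's Hitting reference.
; The DoorMove timeline plays forward or in reverse, offsetting yaw up to 85 degrees from the rotation captured at each toggle.
; The construction script snaps its root to ObjectReference and sets colored open/closed status text.
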(event `self.ReceiveBeginPlay`
  (bind _asbp_first_person_character (cast `/Game/FirstPerson/Blueprints/BP_FirstPersonCharacter` (`GameplayStatics.GetPlayerCharacter` 0)))
  (bind _output_get (set `self.As BP First Person Character` _asbp_first_person_character))
  ;[0 0 0] E Event
  (add `/Game/FirstPerson/Blueprints/BP_FirstPersonCharacter.Interact` _output_get (delegate `DoorStatus`)))

(event `DoorStatus`
  (bind (_original_rotation_roll _original_rotation_pitch _original_rotation_yaw) (`KismetMathLibrary.BreakRotator` (`self.Original Rotation`)))
  (bind _hitting (`/Game/FirstPerson/Blueprints/BP_FirstPersonCharacter.Hitting` (`self.As BP First Person Character`)))
  (bind _returnvalue (`self.K2_GetActorRotation` _hitting))
  (`/Engine/EditorBlueprintResources/StandardMacros.IsValid` _hitting
    (:`Is Valid`
      (if (`self.ActorHasTag` _hitting (`self.Tag`))
        (if (`self.IsOpen`)
          (set `self.Original Rotation` _returnvalue)
          (set `self.IsOpen` false)
          (bind (_direction _newtrack_0) (`Timeline|DoorMove` :!via `ReverseFromEnd` :!label _label)
            (:`Update`
              (if (`self.IsOpen`)
                (`self.K2_SetActorRotation` _hitting (`KismetMathLibrary.MakeRotator` _original_rotation_roll _original_rotation_pitch (+ _original_rotation_yaw (`KismetMathLibrary.Lerp` 0.0 85.0 _newtrack_0))) false)
                (else
                  (`self.K2_SetActorRotation` _hitting (`KismetMathLibrary.MakeRotator` _original_rotation_roll _original_rotation_pitch (+ _original_rotation_yaw (* (`KismetMathLibrary.Lerp` 85.0 0.0 _newtrack_0) -1.0))) false)))))
          (else
            (set `self.Original Rotation` _returnvalue)
            (set `self.IsOpen` true)
            (goto _label :!via `PlayFromStart`)))))))

(fn `TextStatus`
  (params (Value :type Text) (Color :type "Color Structure"))
  (bind _textrender (`self.TextRender`))
  (`TextRenderComponent.K2_SetText` _textrender Value)
  (`TextRenderComponent.K2_SetText` (`self.TextRender1`) Value)
  (`TextRenderComponent.SetTextRenderColor` _textrender Color)
  (`TextRenderComponent.SetTextRenderColor` (`self.TextRender1`) Color)
  (return))

(fn `UserConstructionScript`
  (bind _object_reference (`self.Object Reference`))
  (`|ExecutionSequence`
    (:`then_1`
      ;[0 0 0] PICK DOOR REFERENCE - TELEPORT ACTOR TO DOOR
      (`/Engine/EditorBlueprintResources/StandardMacros.IsValid` _object_reference
        (:`Is Valid`
          (`SceneComponent.K2_SetWorldLocation` (`self.DefaultSceneRoot`) (`self.K2_GetActorLocation` _object_reference) false false))))
    (:`then_2`
      ;[0 0 0] TEXT OPEN / CLOSE
      (if (`self.IsOpen`)
        (`self.TextStatus` "Is open" (make `Color` 0 1))
        (else
          (`self.TextStatus` "Is close" (make `Color` 0 0 1)))))))